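; BP_AICharacter is an enemy AI character that chases the player and kills on contact.
; Pawn sensing sight triggers an AI move to the player, while hearing only prints a message.
; Attack box overlap with the player's hit box waits briefly, then calls the player controller's Die through a DoOnce, reset when overlap ends.
; Its own Die event destroys it and spawns a friendly AI character at its location.
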(event OnSeePawn(PawnSensing)
  (params (Pawn :type Pawn%20Object%20Reference))
  ;[0.15 0.15 0.15 0.5] When AI Character sees the player, calls event to follow the player
  (Variables|Default|SetSaw%20Player true)
  (CallFunction|FollowPlayer))

(event OnHearNoise(PawnSensing)
  (params (Instigator :type Pawn%20Object%20Reference) (Location :type Vector%20%28by%20ref%29 :default "0, 0, 0") (Volume :type Float%20%28single-precision%29))
  (Development|PrintString "I hear you..."))

(event OnComponentBeginOverlap(AttackBox)
  (params (OverlappedComponent :type Primitive%20Component%20Object%20Reference) (OtherActor :type Actor%20Object%20Reference) (OtherComp :type Primitive%20Component%20Object%20Reference) (OtherBodyIndex :type Integer) (bFromSweep :type Boolean) (SweepResult :type Hit%20Result%20Structure%20%28by%20ref%29))
  ;[0.15 0.15 0.15 0.5] Component Overlap for AI Character Attack Box on ThirdPerson Hit Box sets the Overlapped Player and starts a timer with a custom event to attack.
  (bind _asbp_third_person_character (Utilities|Casting|CastToBP_ThirdPersonCharacter OtherActor))
  (if (== (Variables|/Game/ThirdPerson/Blueprints/BP_ThirdPersonCharacter.BP_ThirdPersonCharacter_C|GetHitBox _asbp_third_person_character) OtherComp)
    (Variables|Default|SetOverlapped%20Player _asbp_third_person_character)
    (Utilities|FlowControl|Delay 0.5)
    (Utilities|FlowControl|DoOnce false
      (:Completed
        (bind _asbp_third_person_player_controller (Utilities|Casting|CastToBP_ThirdPersonPlayerController (Game|GetPlayerController 0)))
        (Default|Die _asbp_third_person_player_controller)))))

(event OnComponentEndOverlap(AttackBox)
  (params (OverlappedComponent :type Primitive%20Component%20Object%20Reference) (OtherActor :type Actor%20Object%20Reference) (OtherComp :type Primitive%20Component%20Object%20Reference) (OtherBodyIndex :type Integer))
  ;[0.15 0.15 0.15 0.5] Component End Overlap checks if Overlapped Player is valid, then clears and invalidates the timer before setting the Overlapped Player variable to null.
  (Variables|Default|GetOverlapped%20Player
    (:then
      (bind _asbp_third_person_character (Utilities|Casting|CastToBP_ThirdPersonCharacter OtherActor))
      (if (== (Variables|/Game/ThirdPerson/Blueprints/BP_ThirdPersonCharacter.BP_ThirdPersonCharacter_C|GetHitBox _asbp_third_person_character) OtherComp)
        (Variables|Default|SetOverlapped%20Player 0)
        ;[0.15 0.15 0.15 0.5] Component Overlap for AI Character Attack Box on ThirdPerson Hit Box sets the Overlapped Player and starts a timer with a custom event to attack.
        (Utilities|FlowControl|DoOnce false) ; enters at Reset
      ))
    (:else)))

(event Custom|Follow%20Player
  ;[0.15 0.15 0.15 0.5] Event Follow Player checks if seeing the player then calls AI move to its location
  (if (Variables|Default|GetSaw%20Player)
    (AI|AIMoveTo self "0, 0, 0" (Game|GetPlayerCharacter 0) 5.0 false)))

(event Custom|Die
  ;[0.15 0.15 0.15 0.5] Die event destroys actor
  (Development|PrintString "Destroying...")
  (Actor|DestroyActor)
  (Game|SpawnActorfromClass "/Game/AI/BP_AICharacterFriendly.BP_AICharacterFriendly_C" (Math|Transform|MakeTransform (Transformation|GetActorLocation)) "Undefined" "MultiplyWithRoot" 0 0))

(event EventBeginPlay
  ;[0.15 0.15 0.15 0.5] Event Begin Play sets the Player Character
  (bind _returnvalue (Actor|GetActorOfClass "/Game/ThirdPerson/Blueprints/BP_ThirdPersonCharacter.BP_ThirdPersonCharacter_C"))
  (Variables|Default|SetPlayerCharacter _returnvalue))

(fn ConstructionScript)